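; Rope Blueprint that lays a chosen static mesh along a spline as a chain of deformed spline mesh segments.
; The Construction Script derives section length from mesh length and actor Y scale, then adds Y-forward spline mesh components along the spline.
; Two helper functions supply each segment's local start and end positions and tangents, with tangents clamped to section length.
; The event graph has no runtime logic.
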(event EventBeginPlay)

(event Collision|EventActorBeginOverlap
  (params (OtherActor :type Actor%20Object%20Reference)))

(event EventTick
  (params (DeltaSeconds :type Float%20%28single-precision%29)))

(fn ConstructionScript
  (Variables|Default|SetSection%20Length (* (.y (Transformation|GetActorScale3D)) (Variables|Default|GetMesh%20Length)))
  (for _index (range 0 (Math|Float|Truncate (/ (Spline|GetSplineLength (Variables|Default|GetSpline)) (Variables|Default|GetSection%20Length))))
    (bind _returnvalue (AddComponent|AddSplineMeshComponent false))
    (Components|StaticMesh|SetStaticMesh _returnvalue (Variables|Default|GetStaticMesh))
    (SplineMesh|SetForwardAxis _returnvalue "Y" true)
    (bind (_position _tangent) (CallFunction|GetStartPosition _index))
    (bind (_position_2 _tangent_2) (CallFunction|GetEndPosition _index))
    (SplineMesh|SetStartandEnd _returnvalue _position (Math|Vector|ClampVectorSize _tangent 0.0 (Variables|Default|GetSection%20Length)) _position_2 (Math|Vector|ClampVectorSize _tangent_2 0.0 (Variables|Default|GetSection%20Length)) true :!class /Script/Engine.SplineMeshComponent)))

(fn GetStartPosition
  (params (Index :type Integer))
  (bind _section_length (Variables|Default|GetSection%20Length))
  (bind _spline (Variables|Default|GetSpline))
  (bind _returnvalue (* Index _section_length))
  (return (Spline|GetLocationatDistanceAlongSpline _spline _returnvalue "Local") (Math|Vector|ClampVectorSize (Spline|GetTangentatDistanceAlongSpline _spline _returnvalue "Local") 0.0 (Variables|Default|GetSection%20Length))))

(fn GetEndPosition
  (params (Index :type Integer))
  (bind _returnvalue (+ Index 1))
  (bind _section_length (Variables|Default|GetSection%20Length))
  (bind _spline (Variables|Default|GetSpline))
  (bind _returnvalue_2 (* _returnvalue _section_length))
  (return (Spline|GetLocationatDistanceAlongSpline _spline _returnvalue_2 "Local") (Math|Vector|ClampVectorSize (Spline|GetTangentatDistanceAlongSpline _spline _returnvalue_2 "Local") 0.0 (Variables|Default|GetSection%20Length))))